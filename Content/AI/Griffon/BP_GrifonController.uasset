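; AI controller for the Griffon that starts its BT_Griffon behavior tree on possession and supplies it with the player as a target.
; It stores the first BP_SFDCharacter found in the level in the PlayerActor blackboard key.
; While the SearchForPlayer flag is set, Tick repeats the lookup, and a successful find clears the flag.
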(event EventBeginPlay)

(event EventPossess
  (params (PossessedPawn :type Pawn%20Object%20Reference))
  (AI|RunBehaviorTree "/Game/AI/Griffon/BT_Griffon.BT_Griffon")
  (bind _outactors (Actor|GetAllActorsOfClass "/Game/Player/BP_SFDCharacter.BP_SFDCharacter_C"))
  (if (not (Utilities|Array|IsEmpty _outactors))
    (AI|Components|Blackboard|SetValueasObject (AI|GetBlackboard 0) (Variables|Default|GetPlayerActor) (Utilities|Array|Get(acopy) _outactors))
    (Variables|Default|SetSearchForPlayer false)))

(event EventTick
  (params (DeltaSeconds :type Float%20%28single-precision%29))
  (|CallParentFunction DeltaSeconds)
  (if (Variables|Default|GetSearchForPlayer)
    (bind _outactors (Actor|GetAllActorsOfClass "/Game/Player/BP_SFDCharacter.BP_SFDCharacter_C"))
    (if (not (Utilities|Array|IsEmpty _outactors))
      (AI|Components|Blackboard|SetValueasObject (AI|GetBlackboard 0) (Variables|Default|GetPlayerActor) (Utilities|Array|Get(acopy) _outactors))
      (Variables|Default|SetSearchForPlayer false))))

(fn ConstructionScript)